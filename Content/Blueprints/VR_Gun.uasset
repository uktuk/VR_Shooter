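; A VR gun actor that supports two-handed aiming through separate grip and barrel grab components.
; While both are held, Tick points the actor from the grip hand toward the barrel hand, shifting the target by the grip component's offset from its hand.
; Pitch and yaw come from that look-at, while roll follows the grip hand.
; The grip component's VR interact event calls Fire, whose logic is not defined here.
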(event `self.ReceiveTick`
  (params (DeltaSeconds :type "Float (single-precision)"))
  (bind _currentgrabbedhandtransform (`VR_GrabComponent.CurrentGrabbedHandTransform` (`self.Grip GrabComponent`)))
  (if (`VR_GrabComponent.bIsHeld` (`self.Grip GrabComponent`))
    (if (`VR_GrabComponent.bIsHeld` (`self.Barrel GrabComponent`))
      (`self.K2_SetActorRotation` (`KismetMathLibrary.MakeRotator` (.roll (.rotation _currentgrabbedhandtransform)) (.pitch (`KismetMathLibrary.FindLookAtRotation` (.location _currentgrabbedhandtransform) (+ (.location (`VR_GrabComponent.CurrentGrabbedHandTransform` (`self.Barrel GrabComponent`))) (- (- (`SceneComponent.K2_GetComponentLocation` (`self.Barrel GrabComponent`)) (.location (`VR_GrabComponent.CurrentGrabbedHandTransform` (`self.Grip GrabComponent`)))) (- (`SceneComponent.K2_GetComponentLocation` (`self.Barrel GrabComponent`)) (`SceneComponent.K2_GetComponentLocation` (`self.Grip GrabComponent`))))))) (.yaw (`KismetMathLibrary.FindLookAtRotation` (.location _currentgrabbedhandtransform) (+ (.location (`VR_GrabComponent.CurrentGrabbedHandTransform` (`self.Barrel GrabComponent`))) (- (- (`SceneComponent.K2_GetComponentLocation` (`self.Barrel GrabComponent`)) (.location (`VR_GrabComponent.CurrentGrabbedHandTransform` (`self.Grip GrabComponent`)))) (- (`SceneComponent.K2_GetComponentLocation` (`self.Barrel GrabComponent`)) (`SceneComponent.K2_GetComponentLocation` (`self.Grip GrabComponent`))))))))))))

(event `self.Grip GrabComponent.OnVRInteract_delegate`
  (`self.Fire`))

(fn `UserConstructionScript`)