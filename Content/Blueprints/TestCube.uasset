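; TestCube is a grabbable sliding drawer that follows the grabbing hand along a single axis.
; BeginPlay stores the drawer's origin; while HandleGrabComponent is held, Tick measures the hand's offset from that origin, compensating for the handle and right-hand attach point.
; It projects that offset onto MoveDirection rotated into world space, clamps its length between MinDistance and MaxDistance, and moves the drawer there without sweeping.
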(event `self.ReceiveBeginPlay`
  (set `self.DrawerOrigin` (`SceneComponent.K2_GetComponentLocation` (`self.Drawer`))))

(event `self.ReceiveTick`
  (params (DeltaSeconds :type "Float (single-precision)"))
  (if (`VR_GrabComponent.bIsHeld` (`self.HandleGrabComponent`))
    (bind _returnvalue (`self.Get Vector from drawer origin to MC transform`))
    (`SceneComponent.K2_SetWorldLocation` (`self.Drawer`) (+ (`KismetMathLibrary.ClampVectorSize` (`KismetMathLibrary.ProjectVectorOnToVector` _returnvalue (`KismetMathLibrary.GreaterGreater_VectorRotator` (`self.MoveDirection`) (`SceneComponent.K2_GetComponentRotation` (`self.Drawer`)))) (`self.MinDistance`) (`self.MaxDistance`)) (`self.DrawerOrigin`)) false false)))

(fn `Get Vector from drawer origin to MC transform`
  (returns (ReturnValue :type "Vector Structure"))
  (bind _handlegrabcomponent (`self.HandleGrabComponent`))
  (return (- (.location (`VR_GrabComponent.CurrentGrabbedHandTransform` (`self.HandleGrabComponent`))) (+ (`self.DrawerOrigin`) (- (- (`SceneComponent.K2_GetComponentLocation` _handlegrabcomponent) (* (`SceneComponent.K2_GetComponentScale` (`self.HandleGrabComponent`)) (.location (`VR_GrabComponent.AttachPointTransformForRightHand` _handlegrabcomponent)))) (`SceneComponent.K2_GetComponentLocation` (`self.Drawer`)))))))

(fn `UserConstructionScript`)