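; Gun Blueprint that handles magazine eject and insert, with no firing logic.
; DropMag and PickupMag input presses call OnClipEject and OnClipInsert.
; Eject detaches the Magazine component, keeping its world transform.
; Insert makes a snap-to-target, welded attach call that names Magazine as the parent, not as the component being attached.
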(event `InputAction|DropMag`
  (params (Key :type "Key Structure" :default "AnyKey"))
  (:`Pressed`
    (`self.On Clip Eject`)))

(event `InputAction|PickupMag`
  (params (Key :type "Key Structure" :default "AnyKey"))
  (:`Pressed`
    (`self.On Clip Insert`)))

(event `On Clip Eject`
  (`SceneComponent.K2_DetachFromComponent` (`self.Magazine`) "KeepWorld" "KeepWorld" "KeepWorld" true))

(event `On Clip Insert`
  (`self.K2_AttachToComponent` (`self.Magazine`) "None" "SnapToTarget" "SnapToTarget" "SnapToTarget" true))

(fn `UserConstructionScript`)