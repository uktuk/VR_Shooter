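; Weapon Blueprint that fires projectiles and accepts snap-on magazines.
; The FireWeapon input calls Fire, which spawns the projectile class at the mesh's muzzle socket, with no ammo or magazine check.
; A WeaponMagazine overlapping the reload capsule is attached to the weapon, snapped to the clip socket.
; HasMagazine is an unused stub that always returns false.
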(event `InputAction|FireWeapon`
  (params (Key :type "Key Structure" :default "AnyKey"))
  (:`Pressed`
    (`self.Fire`)))

(event `self.ReloadMagCapsule.OnComponentBeginOverlap`
  (params (OverlappedComponent :type "PrimitiveComponent Object Reference") (OtherActor :type "Actor Object Reference") (OtherComp :type "PrimitiveComponent Object Reference") (OtherBodyIndex :type Integer) (bFromSweep :type Boolean) (SweepResult :type "HitResult Structure (by ref)"))
  ;[1 1 1] Snap any magazine that overlaps the capsule location.
  (bind _asweapon_magazine (cast `/Game/Imported/Blueprint/WeaponMagazine` OtherActor))
  (`self.AttachMag` _asweapon_magazine))

(fn `AttachMag`
  (params (NewMagActor :type "Actor Object Reference"))
  (`self.K2_AttachToActor` NewMagActor self (`self.ClipLocation`) "SnapToTarget" "SnapToTarget" "SnapToTarget" false))

(fn `Fire`
  (`|SpawnActorFromClass` (`GameplayStatics.GetObjectClass` (`self.ProjectileClass`)) (`SceneComponent.GetSocketTransform` (`self.WeaponMesh`) (`self.MuzzleLocation`) "RTS_World") "AlwaysSpawn" "OverrideRootScale"))

(fn `HasMagazine`
  (returns (bHasMag :type Boolean))
  (return false))

(fn `UserConstructionScript`)